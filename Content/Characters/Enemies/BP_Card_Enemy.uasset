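; BP_Card_Enemy is an enemy that turns toward and attacks the third-person player character when its PawnSensing component sees it.
; It yaws to face the player by aiming the look-at at its own height.
; When CanAttack is set, it spawns a BP_Projectile at SpawnLocation and applies damage to the player immediately, independent of any projectile hit.
; A delay then re-enables CanAttack, acting as the attack cooldown.
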(event OnSeePawn(PawnSensing)
  (params (Pawn :type Pawn%20Object%20Reference))
  (bind _returnvalue (Transformation|GetActorLocation Pawn))
  (bind _asbp_third_person_character (Utilities|Casting|CastToBP_ThirdPersonCharacter Pawn))
  (Transformation|SetActorRotation (Math|Rotator|FindRelativeLookatRotation (Math|Conversions|ToTransform(Vector) (Transformation|GetActorLocation)) (Math|Vector|MakeVector (.x _returnvalue) (.y _returnvalue) (.z (Transformation|GetActorLocation)))))
  (if (Variables|Default|GetCanAttack)
    (Game|SpawnActorfromClass "/Game/ThirdPerson/Blueprints/BP_Projectile.BP_Projectile_C" (Transformation|GetWorldTransform (Variables|Default|GetSpawn%20Location)) "Undefined" "MultiplyWithRoot" 0 0)
    (Game|Damage|ApplyDamage _asbp_third_person_character 1.0 0 0)
    (Variables|Default|SetCanAttack false)
    (Utilities|FlowControl|Delay 2.0)
    (Variables|Default|SetCanAttack true)))

(event EventBeginPlay)

(event Collision|EventActorBeginOverlap
  (params (OtherActor :type Actor%20Object%20Reference)))

(event EventTick
  (params (DeltaSeconds :type Float%20%28single-precision%29)))

(fn ConstructionScript)